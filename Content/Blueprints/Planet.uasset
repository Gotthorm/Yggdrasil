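; Planet Blueprint actor that represents a celestial body as a sphere, sized and placed from real-world-scale values.
; The construction script divides the kilometer radius by a celestial unit factor, doubles it for the sphere's world scale, and divides the celestial position by the same factor for its world location.
; The event graph holds no active logic, so all setup happens at construction.
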(fn `UserConstructionScript`
  (`SceneComponent.SetWorldScale3D` (`self.Sphere`) (`KismetMathLibrary.Conv_DoubleToVector` (* (/ (`self.Kilometer Radius`) (`self.CelestialUnits`)) 2.0)))
  (`SceneComponent.K2_SetWorldLocation` (`self.Sphere`) (/ (`self.Celestial Position`) (`self.CelestialUnits`)) false false))